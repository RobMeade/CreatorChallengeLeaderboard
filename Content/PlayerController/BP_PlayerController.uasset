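; Player controller that runs the main menu and leaderboard UI, switches input between menu and game, and tracks the player's score.
; BeginPlay fires a player-controlled-initialized dispatcher, while separate init functions set up either menu or game mode.
; Menu setup creates both widgets, binds their buttons to open ThirdPersonMap, swap visible screens or quit, and sets UI-only input.
; IncrementScore raises the score and broadcasts the change through a dispatcher.
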(event `self.ReceiveBeginPlay`
  ;[1 1 1] Initialize
  (`self.PlayerControlledInitialized`))

(fn `BindToEventsForMainMenu`
  ;[1 1 1] Bind to Main Menu Events
  (add `/Game/UI/WBP_MainMenu.PlayButtonClicked` (`self.MainMenuWidget`) (`|CreateDelegate` :!event `OnMainMenuPlayButtonClicked`))
  (add `/Game/UI/WBP_MainMenu.LeaderboardButtonClicked` (`self.MainMenuWidget`) (`|CreateDelegate` :!event `OnMainMenuLeaderboardButtonClicked`))
  (add `/Game/UI/WBP_MainMenu.QuitButtonClicked` (`self.MainMenuWidget`) (`|CreateDelegate` :!event `OnMainMenuQuitButtonClicked`))
  (add `/Game/UI/WBP_Leaderboard.MainMenuButtonClicked` (`self.LeaderboardWidget`) (`|CreateDelegate` :!event `OnLeaderboardMainMenuClicked`)))

(fn `CreateUIWidgetsForMainMenu`
  ;[1 1 1] Creates the user interface widgets
  (bind _returnvalue (`|CreateWidget` "/Game/UI/WBP_MainMenu.WBP_MainMenu_C"))
  (bind _output_get (set `self.MainMenuWidget` _returnvalue))
  (`UserWidget.AddToViewport` _output_get 0)
  (bind _returnvalue_2 (`|CreateWidget` "/Game/UI/WBP_Leaderboard.WBP_Leaderboard_C"))
  (bind _output_get_2 (set `self.LeaderboardWidget` _returnvalue_2))
  (`UserWidget.AddToViewport` _output_get_2 0)
  (`self.ToggleWidgetVisibility` (`self.LeaderboardWidget`)))

(fn `IncrementScore`
  ;[1 1 1] Increment Score
  (`/Engine/EditorBlueprintResources/StandardMacros.IncrementInt` (`self.Score`)
    (:`  `
      (`self.PlayerScoreChanged` (`self.Score`)))))

(fn `InitializeForGame`
  ;[1 1 1] Initialize for Game
  (`self.SetInputModeForGame`))

(fn `InitializeForMainMenu`
  ;[1 1 1] Initialize for Main Menu
  (`self.CreateUIWidgetsForMainMenu`)
  (`self.BindToEventsForMainMenu`)
  (`self.SetInputModeForMenu`))

(fn `OnLeaderboardMainMenuClicked`
  ;[1 1 1] Leaderboard - Main Menu Button Clicked
  (`self.ToggleWidgetVisibility` (`self.LeaderboardWidget`))
  (`self.ToggleWidgetVisibility` (`self.MainMenuWidget`)))

(fn `OnMainMenuLeaderboardButtonClicked`
  ;[1 1 1] Main Menu - Leaderboard Button Clicked
  (`self.ToggleWidgetVisibility` (`self.MainMenuWidget`))
  (`self.ToggleWidgetVisibility` (`self.LeaderboardWidget`)))

(fn `OnMainMenuPlayButtonClicked`
  ;[1 1 1] Main Menu - Play Button Clicked
  (`Widget.RemoveFromParent` (`self.MainMenuWidget`))
  (`GameplayStatics.OpenLevel` "ThirdPersonMap"))

(fn `OnMainMenuQuitButtonClicked`
  ;[1 1 1] Main Menu - Quit Button Clicked
  (`KismetSystemLibrary.QuitGame` null "Quit"))

(fn `SetInputModeForGame`
  ;[1 1 1] Set Input Mode for Game
  (`WidgetBlueprintLibrary.SetInputMode_GameOnly` self)
  (set `self.bShowMouseCursor` false))

(fn `SetInputModeForMenu`
  ;[1 1 1] Set Input Mode for Menu
  (`WidgetBlueprintLibrary.SetInputMode_UIOnlyEx` self (`self.MainMenuWidget`))
  (set `self.bShowMouseCursor` true))

(fn `ToggleWidgetVisibility`
  (params (Widget :type "UserWidget Object Reference"))
  (locals (NewLocalVar :type "UserWidget Object Reference"))
  ;[1 1 1] Toggles the widgets visibilty (show/hide)
  (`Widget.SetVisibility` (`local.Widget`) (select `ESlateVisibility` (`Widget.GetVisibility` Widget) :`Visible` "Hidden" :`Collapsed` "SelfHitTestInvisible" :`Hidden` "SelfHitTestInvisible" :`HitTestInvisible` "Hidden" :`SelfHitTestInvisible` "Hidden" :!type "ESlateVisibility Enum")))

(fn `UserConstructionScript`)