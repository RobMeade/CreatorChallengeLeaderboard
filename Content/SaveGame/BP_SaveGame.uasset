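; BP_SaveGame is a save game object that persists the TopScores high-score data to a named slot.
; LoadData copies TopScores from the saved slot into itself and returns it, or first writes itself to the slot when no save exists.
; Initialize sets TopScores in memory, while SaveData sets it and immediately writes the object to the slot.
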(fn `Initialize`
  (params (TopScores :type "Array of TopScore Structure"))
  ;[1 1 1] Initialize
  (set `self.TopScores` TopScores))

(fn `LoadData`
  (returns (TopScores :type "Array of TopScore Structure"))
  ;[1 1 1] Load Data
  (bind _returnvalue (`GameplayStatics.DoesSaveGameExist` (`self.SlotName`)))
  (if _returnvalue
    (bind _returnvalue_2 (`GameplayStatics.LoadGameFromSlot` (`self.SlotName`)))
    (bind _asbp_save_game (cast `/Game/SaveGame/BP_SaveGame` _returnvalue_2))
    (set `self.TopScores` (`/Game/SaveGame/BP_SaveGame.TopScores` _asbp_save_game))
    (else
      (`GameplayStatics.SaveGameToSlot` self (`self.SlotName`))))
  (return (`self.TopScores`)))

(fn `SaveData`
  (params (TopScores :type "Array of TopScore Structure"))
  ;[1 1 1] Save Data
  (set `self.TopScores` TopScores)
  (`GameplayStatics.SaveGameToSlot` self (`self.SlotName`)))