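; BP_Spawner is an actor that drops physics-simulated BP_Target actors at random points inside its box bounds on a looping one-second timer.
; It relays each target's self-destruct through its own event dispatcher.
; It binds to BP_GameMode_Game's game-over event and clears the spawn timer when the game ends.
; An EndGame event that disables player input remains, but its timer is never run.
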(event `EndGame`
  ;[1 1 1] End Game
  (`self.DisableInput` (`GameplayStatics.GetPlayerPawn` 0) (`GameplayStatics.GetPlayerController` 0))
  (`KismetSystemLibrary.PrintString` "Game Over" true true (struct :`R` 1.0 :`G` 0.016463 :`A` 1.0) 10.0))

(event `self.ReceiveBeginPlay`
  (`self.SetReferences`)
  (`self.BindToEvents`)
  (`KismetSystemLibrary.Delay` 0.2)
  (bind _returnvalue (`KismetSystemLibrary.K2_SetTimerDelegate` (delegate `SpawnGOG`) 1.0 true))
  (set `self.TargetSpawnTimerHandle` _returnvalue))

(event `SpawnGOG`
  (bind (_origin _boxextent) (`KismetSystemLibrary.GetComponentBounds` (`self.Box`)))
  ;[1 1 1] SpawnGiftsFromGod
  (bind _returnvalue (`|SpawnActorFromClass` "/Game/Blueprints/BP_Target.BP_Target_C" (`KismetMathLibrary.MakeTransform` (`KismetMathLibrary.RandomPointInBoundingBox` _origin _boxextent)) "Undefined" "OverrideRootScale" null null))
  (`PrimitiveComponent.SetSimulatePhysics` (`/Game/Blueprints/BP_Target.StaticMesh` _returnvalue) true)
  (add `/Game/Blueprints/BP_Target.SelfDestructInitiated` _returnvalue (`|CreateDelegate` :!event `OnTargetSelfDestructInitiated`)))

(fn `BindToEvents`
  ;[1 1 1] Bind to Events
  (add `/Game/GameModes/BP_GameMode_Game.GameOverStateChanged` (`self.GameModeGame`) (`|CreateDelegate` :!event `OnGameOverStateChanged`)))

(fn `OnGameOverStateChanged`
  (params (bGameIsOver :type Boolean))
  ;[1 1 1] Game Over State Changed
  (if bGameIsOver
    (`KismetSystemLibrary.K2_ClearAndInvalidateTimerHandle` (`self.TargetSpawnTimerHandle`))))

(fn `OnTargetSelfDestructInitiated`
  ;[1 1 1] Target Self Destruct Initiated
  (`self.TargetSelfDestructInitiated`))

(fn `SetReferences`
  ;[1 1 1] Set References
  (bind _asbp_game_mode_game (cast `/Game/GameModes/BP_GameMode_Game` (`GameplayStatics.GetGameMode`)))
  (set `self.GameModeGame` _asbp_game_mode_game))

(fn `UserConstructionScript`)