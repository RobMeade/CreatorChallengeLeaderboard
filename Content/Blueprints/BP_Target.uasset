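; BP_Target is a destructible barrel target that explodes when hit by a bullet.
; On BeginPlay it gives its static mesh a random model from the Barrels array.
; When a BP_Bullet overlaps its Box component, it spawns an explosion particle and sound at the mesh location, then destroys itself.
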(event `self.ReceiveBeginPlay`
  ;[1 1 1] Set Random Static Mesh from Barrels Mesh array
  (`StaticMeshComponent.SetStaticMesh` (`self.StaticMesh`) (`KismetArrayLibrary.Array_Random` (`self.Barrels`))))

(event `self.Box.OnComponentBeginOverlap`
  (params (OverlappedComponent :type "PrimitiveComponent Object Reference") (OtherActor :type "Actor Object Reference") (OtherComp :type "PrimitiveComponent Object Reference") (OtherBodyIndex :type Integer) (bFromSweep :type Boolean) (SweepResult :type "HitResult Structure (by ref)"))
  (bind _returnvalue (`SceneComponent.K2_GetComponentLocation` (`self.StaticMesh`)))
  ;[1 1 1] Die when hit by Bullet
  (cast `/Game/Blueprints/BP_Bullet` OtherActor)
  (`GameplayStatics.SpawnEmitterAtLocation` "/Game/StarterContent/Particles/P_Explosion.P_Explosion" _returnvalue)
  (`GameplayStatics.PlaySoundAtLocation` "/Game/StarterContent/Audio/Explosion_Cue.Explosion_Cue" _returnvalue (struct) 1.0 1.0 0.0 null null null null)
  (`self.K2_DestroyActor`))

(fn `UserConstructionScript`)