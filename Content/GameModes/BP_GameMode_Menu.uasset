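; Game mode for the main menu that prepares the player controller for menu use.
; On BeginPlay it caches player 0's BP_PlayerController and binds to that controller's initialized event.
; Its OnPlayerControllerInitialized handler calls InitializeForMainMenu on the cached controller.
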(event `self.ReceiveBeginPlay`
  ;[1 1 1] Initialize
  (`self.SetReferences`)
  (`self.BindToEvents`))

(fn `BindToEvents`
  ;[1 1 1] Bind to Events
  (add `/Game/PlayerController/BP_PlayerController.PlayerControlledInitialized` (`self.PlayerController`) (`|CreateDelegate` :!event `OnPlayerControllerInitialized`)))

(fn `OnPlayerControllerInitialized`
  ;[1 1 1] Player controller initialized
  (`/Game/PlayerController/BP_PlayerController.InitializeForMainMenu` (`self.PlayerController`)))

(fn `SetReferences`
  ;[1 1 1] Set references
  (bind _asbp_player_controller (cast `/Game/PlayerController/BP_PlayerController` (`GameplayStatics.GetPlayerController` 0)))
  (set `self.PlayerController` _asbp_player_controller))

(fn `UserConstructionScript`)