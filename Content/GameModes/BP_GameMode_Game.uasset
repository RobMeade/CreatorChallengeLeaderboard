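; Game mode for gameplay that links the player controller, target spawners and score.
; On BeginPlay it caches the first player controller and all BP_Spawner actors, then binds to their events.
; It initializes the controller for the game once that reports ready and increments score when a spawner reports a target self-destruct.
; Score changes from the controller are re-broadcast through the game mode's own PlayerScoreChanged call.
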(event `self.ReceiveBeginPlay`
  ;[1 1 1] Initialize
  (`self.SetReferences`)
  (`self.BindToEvents`))

(fn `BindToEvents`
  ;[1 1 1] Bind to Events
  (add `/Game/PlayerController/BP_PlayerController.PlayerControlledInitialized` (`self.PlayerController`) (`|CreateDelegate` :!event `OnPlayerControllerInitialized`))
  (add `/Game/PlayerController/BP_PlayerController.PlayerScoreChanged` (`self.PlayerController`) (`|CreateDelegate` :!event `OnPlayerScoreChanged`))
  (for _array_element (`self.Spawners`)
    (add `/Game/Blueprints/BP_Spawner.TargetSelfDestructInitiated` _array_element (`|CreateDelegate` :!event `OnTargetSelfDestructInitiated`))))

(fn `OnPlayerControllerInitialized`
  ;[1 1 1] Player controller initialized
  (`/Game/PlayerController/BP_PlayerController.InitializeForGame` (`self.PlayerController`)))

(fn `OnPlayerScoreChanged`
  (params (Score :type Integer))
  ;[1 1 1] Player Score Changed
  (`self.PlayerScoreChanged` Score))

(fn `OnTargetSelfDestructInitiated`
  ;[1 1 1] Target destroyed, increment player score
  (`/Game/PlayerController/BP_PlayerController.IncrementScore` (`self.PlayerController`)))

(fn `SetReferences`
  ;[1 1 1] Set references
  (bind _asbp_player_controller (cast `/Game/PlayerController/BP_PlayerController` (`GameplayStatics.GetPlayerController` 0)))
  (set `self.PlayerController` _asbp_player_controller)
  (bind _outactors (`GameplayStatics.GetAllActorsOfClass` "/Game/Blueprints/BP_Spawner.BP_Spawner_C"))
  (set `self.Spawners` _outactors))

(fn `UserConstructionScript`)